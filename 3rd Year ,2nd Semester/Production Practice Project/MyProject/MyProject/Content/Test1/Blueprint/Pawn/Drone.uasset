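; Flying AI drone Character that hovers at FlyHeight above traced ground and travels along waypoints, pausing at each.
; NewPoint builds a route with SearchRoad, a recursive capsule-trace search that fans out around obstacles, then ReverseSearch reverses and shortcuts it.
; Tick interpolates height and steers horizontally along that route, or along CustomPoints when CustomMoving is set.
; The older Moving logic, mesh tilt and bob animation are disconnected.
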(event `self.ReceiveBeginPlay`
  (`KismetSystemLibrary.Delay` 2.0)
  (`self.StartAI`)
  (`self.FindLocation`))

(event `PlayFlyingAnim`)

(event `self.ReceiveTick`
  (params (DeltaSeconds :type "Float (single-precision)"))
  (`self.Flying`))

(event `StartAI`
  (`CharacterMovementComponent.SetMovementMode` (`self.CharacterMovement`) "MOVE_Flying" 0)
  (set `self.Enabled` true))

(event `StopFlyingAnim`
  (if (`TimelineComponent.IsPlaying` (`self.Animation`))
    (`TimelineComponent.Stop` (`self.Animation`))))

(event `Flying`
  (bind (_returnvalue_x _returnvalue_y _returnvalue_z) (`KismetMathLibrary.BreakVector` (`self.K2_GetActorLocation`)))
  (bind (_returnvalue_x_2 _returnvalue_y_2 _returnvalue_z_2) (`KismetMathLibrary.BreakVector` (`self.K2_GetActorLocation`)))
  (bind (_returnvalue_x_3 _returnvalue_y_3) (`KismetMathLibrary.BreakVector` (`self.K2_GetActorLocation`)))
  (bind _currenttargetindex (`self.CurrentTargetIndex`))
  (bind (_currenttarget_x _currenttarget_y) (`KismetMathLibrary.BreakVector` (`self.CurrentTarget`)))
  (bind _custompoints (`self.CustomPoints`))
  (bind (_rotation _location) (break `/Game/Test1/Blueprint/Data/Str_Point` (`|GetArrayItem` _custompoints _currenttargetindex)))
  (bind (_returnvalue_x_4 _returnvalue_y_4) (`KismetMathLibrary.BreakVector` (`KismetMathLibrary.GetForwardVector` (`KismetMathLibrary.FindLookAtRotation` (`self.K2_GetActorLocation`) (`self.CurrentTarget`)))))
  (`|ExecutionSequence`
    (:`then_0`
      (bind (_landfound _distance _traceend) (`self.fCheckHeight`))
      (bind _returnvalue (+ (.z _traceend) (`self.FlyHeight`)))
      (`self.K2_SetActorLocation` (`KismetMathLibrary.MakeVector` _returnvalue_x _returnvalue_y (`KismetMathLibrary.FInterpTo` _returnvalue_z _returnvalue (`GameplayStatics.GetWorldDeltaSeconds`) 1.0)))
      (if (`KismetMathLibrary.NearlyEqual_FloatFloat` _returnvalue_z_2 _returnvalue 150.0)
        (`self.PlayFlyingAnim`)
        (set `self.IsActualHeight` true)
        (else
          (`self.StopFlyingAnim`)
          (set `self.IsActualHeight` false))))
    (:`then_1`
      (if (`self.IsMoving`)
        (`self.AddMovementInput` (`KismetMathLibrary.MakeVector` _returnvalue_x_4 _returnvalue_y_4))
        (if (== (`KismetMathLibrary.MakeVector` _returnvalue_x_3 _returnvalue_y_3) (`KismetMathLibrary.MakeVector` _currenttarget_x _currenttarget_y) :`ErrorTolerance` 100.0)
          (`/Engine/EditorBlueprintResources/StandardMacros.IncrementInt` (`self.CurrentTargetIndex`)
            (:`  `
              (if (`self.CustomMoving`)
                (if (!= (`KismetArrayLibrary.Array_Length` _custompoints) _currenttargetindex)
                  (set `self.CurrentTarget` _location)
                  (set `CharacterMovementComponent.bOrientRotationToMovement` _rotation (`self.CharacterMovement`))
                  (set `self.IsMoving` false :!label _label)
                  (`KismetSystemLibrary.Delay` (`self.DelayTime`))
                  (set `self.IsMoving` true)
                  (else
                    (set `self.IsMoving` false :!label _label_2)))
                (elif (!= (`KismetArrayLibrary.Array_Length` (`self.PointLocations`)) _currenttargetindex)
                  (set `self.CurrentTarget` (`|GetArrayItem` (`self.PointLocations`) _currenttargetindex))
                  (goto _label)
                  (else
                    (goto _label_2)))))))))))

(event `NewPoint`
  (params (Location :type "Vector Structure"))
  (if (not (`self.CustomMoving`))
    (`KismetArrayLibrary.Array_Clear` (`self.PointLocations`))
    (bind _success (`self.SearchRoad` (`self.K2_GetActorLocation`) Location 0 (`self.K2_GetActorRotation`)))
    (if _success
      (`self.ReverseSearch`)
      (`KismetArrayLibrary.Array_Add` (`self.PointLocations`) Location)
      (`self.StartMove`))
    (else
      (`self.StartMove`))))

(event `StartMove`
  (bind _pointlocations (`self.PointLocations`))
  (bind (_rotation _location) (break `/Game/Test1/Blueprint/Data/Str_Point` (`|GetArrayItem` (`self.CustomPoints`))))
  (if (and (`self.Enabled`) (`self.IsActualHeight`))
    (if (not (`self.CustomMoving`))
      (if (> (`KismetArrayLibrary.Array_Length` _pointlocations) 0)
        (set `self.CurrentTargetIndex` 0)
        (set `self.CurrentTarget` (`|GetArrayItem` _pointlocations))
        (set `self.IsMoving` true))
      (elif (> (`KismetArrayLibrary.Array_Length` (`self.CustomPoints`)) 0)
        (set `self.CurrentTargetIndex` 0)
        (set `self.CurrentTarget` _location)
        (set `CharacterMovementComponent.bOrientRotationToMovement` _rotation (`self.CharacterMovement`))
        (set `self.IsMoving` true)))))

(fn `fCheckHeight`
  (returns (LandFound :type Boolean) (Distance :type "Float (double-precision)") (TraceEnd :type "Vector Structure"))
  (bind (_outhit _returnvalue) (`KismetSystemLibrary.LineTraceSingle` (`self.K2_GetActorLocation`) (- (`self.K2_GetActorLocation`) (0.0 0.0 2000.0)) "TraceTypeQuery2"))
  (bind (_bblockinghit _binitialoverlap _time _distance _location _impactpoint) (`GameplayStatics.BreakHitResult` _outhit))
  (return (and _returnvalue _bblockinghit) _distance _impactpoint))

(fn `FindAdditionalLocation`
  (locals (Locations :type "Array of Vector Structure"))
  (bind _returnvalue (`self.K2_GetActorLocation`))
  (for _index (range 1 9)
    (`|ExecutionSequence`
      (:`then_0`
        (bind _returnvalue_2 (`KismetMathLibrary.Conv_IntToDouble` _index))
        (bind (_outhit _returnvalue_3) (`KismetSystemLibrary.CapsuleTraceSingle` :`Start` _returnvalue :`End` (+ _returnvalue (* (`KismetMathLibrary.RotateAngleAxis` (`KismetMathLibrary.GetForwardVector` (`KismetMathLibrary.FindLookAtRotation` (`self.K2_GetActorLocation`) (`self.FinalLocation`))) (* _returnvalue_2 15.0) (`self.GetActorUpVector`)) (`self.FindDist`))) :`Radius` 50.0 :`HalfHeight` 50.0 :`TraceChannel` "TraceTypeQuery1" :`DrawDebugType` "ForOneFrame" :`DrawTime` 3.0))
        (if (not _returnvalue_3)
          (bind (_bblockinghit _binitialoverlap _time _distance _location _impactpoint _normal _impactnormal _physmat _hitactor _hitcomponent _hitbonename _hititem _faceindex _tracestart _traceend) (`GameplayStatics.BreakHitResult` _outhit))
          (set `self.TargetLocation` _traceend)
          (return)
          (else
            (`KismetArrayLibrary.Array_Add` (`local.Locations`) _impactpoint))))
      (:`then_1`
        (bind (_outhit_2 _returnvalue_4) (`KismetSystemLibrary.CapsuleTraceSingle` :`Start` _returnvalue :`End` (+ (`self.K2_GetActorLocation`) (* (`KismetMathLibrary.RotateAngleAxis` (`KismetMathLibrary.GetForwardVector` (`KismetMathLibrary.FindLookAtRotation` (`self.K2_GetActorLocation`) (`self.FinalLocation`))) (* _returnvalue_2 -15.0) (`self.GetActorUpVector`)) (`self.FindDist`))) :`Radius` 50.0 :`HalfHeight` 50.0 :`TraceChannel` "TraceTypeQuery1" :`DrawDebugType` "ForOneFrame" :`DrawTime` 3.0))
        (if (not _returnvalue_4)
          (bind (_bblockinghit_2 _binitialoverlap_2 _time_2 _distance_2 _location_2 _impactpoint_2 _normal_2 _impactnormal_2 _physmat_2 _hitactor_2 _hitcomponent_2 _hitbonename_2 _hititem_2 _faceindex_2 _tracestart_2 _traceend_2) (`GameplayStatics.BreakHitResult` _outhit_2))
          (set `self.TargetLocation` _traceend_2)
          (return)
          (else
            (`KismetArrayLibrary.Array_Add` (`local.Locations`) _impactpoint_2)))))))

(fn `FindLocation`
  (returns (Success :type Boolean))
  (locals (NewLocalVar_0 :type "Array of /Game/Test1/Blueprint/Objects/Point Object Reference"))
  (bind _newlocalvar_0 (`local.NewLocalVar_0`))
  (bind _outactors (`GameplayStatics.GetAllActorsOfClass` "/Game/Test1/Blueprint/Objects/Point.Point_C"))
  (set `local.NewLocalVar_0` _outactors)
  (`self.GetNear` _newlocalvar_0)
  (if (> (`KismetArrayLibrary.Array_Length` _newlocalvar_0) 0)
    (set `self.FinalLocation` (`self.K2_GetActorLocation` (`|GetArrayItem` (`local.NewLocalVar_0`))))
    (set `self.CanMove` true)
    (set `self.Enabled` true)
    (`CharacterMovementComponent.SetMovementMode` (`self.CharacterMovement`) "MOVE_Flying" 0)
    (return true)
    (else
      (return false))))

(fn `GetLinecolor`
  (params (Index :type Integer))
  (returns (Color :type "LinearColor Structure"))
  (if (>= Index 10)
    (return (struct :`R` 1.0 :`B` 1.0 :`A` 1.0))
    (else
      (return (select `int` Index :`0` (struct :`R` 1.0 :`G` 1.0 :`A` 1.0) :`1` (struct :`R` 1.0 :`G` 0.8 :`A` 1.0) :`2` (struct :`R` 1.0 :`G` 0.6 :`A` 1.0) :`3` (struct :`R` 1.0 :`G` 0.4 :`A` 1.0) :`4` (struct :`R` 1.0 :`G` 0.2 :`A` 1.0) :`5` (struct :`R` 1.0 :`A` 1.0) :`6` (struct :`R` 1.0 :`B` 0.2 :`A` 1.0) :`7` (struct :`R` 1.0 :`B` 0.4 :`A` 1.0) :`8` (struct :`R` 1.0 :`B` 0.6 :`A` 1.0) :`9` (struct :`R` 1.0 :`B` 0.8 :`A` 1.0) :!type "LinearColor Structure")))))

(fn `GetNear`
  (params (Array :type "Array of Actor Object Reference (by ref)"))
  (locals (Index :type Integer) (Dist :type "Float (double-precision)"))
  (bind _returnvalue (`self.K2_GetActorLocation`))
  (for (_array_element _array_index) Array
    (for (_array_element_2 _array_index_2) Array
      (if (!= _array_index _array_index_2)
        (if (> (`KismetMathLibrary.Vector_Distance2D` (`self.K2_GetActorLocation` _array_element_2) _returnvalue) (`KismetMathLibrary.Vector_Distance2D` _returnvalue (`self.K2_GetActorLocation` _array_element)))
          (`KismetArrayLibrary.Array_Swap` Array _array_index_2 _array_index))))))

(fn `Move`
  (bind (_returnvalue_x _returnvalue_y) (`KismetMathLibrary.BreakVector` (`self.K2_GetActorLocation`)))
  (bind (_currenttarget_x _currenttarget_y) (`KismetMathLibrary.BreakVector` (`self.CurrentTarget`)))
  (bind (_returnvalue_x_2 _returnvalue_y_2) (`KismetMathLibrary.BreakVector` (`KismetMathLibrary.GetForwardVector` (`KismetMathLibrary.FindLookAtRotation` (`self.K2_GetActorLocation`) (`self.CurrentTarget`)))))
  (if (not (`self.IsMoving`))
    (return)
    (else
      (`self.AddMovementInput` (`KismetMathLibrary.MakeVector` _returnvalue_x_2 _returnvalue_y_2))
      (if (== (`KismetMathLibrary.MakeVector` _returnvalue_x _returnvalue_y) (`KismetMathLibrary.MakeVector` _currenttarget_x _currenttarget_y) :`ErrorTolerance` 100.0)
        (bind _result (`/Engine/EditorBlueprintResources/StandardMacros.IncrementInt` (`self.CurrentTargetIndex`)))))))

(fn `ReverseSearch`
  (locals (nLoc :type "Array of Vector Structure") (IgnoreActors :type "Array of Actor Object Reference"))
  (bind (_outradius _outhalfheight) (`CapsuleComponent.GetScaledCapsuleSize` (`self.CapsuleComponent`)))
  (`KismetArrayLibrary.Array_Clear` (`local.nLoc`))
  (if (> (`KismetArrayLibrary.Array_Length` (`self.PointLocations`)) 0)
    (`|ExecutionSequence`
      (:`then_0`
        (`KismetArrayLibrary.Array_Clear` (`local.IgnoreActors`))
        (bind _outactors (`GameplayStatics.GetAllActorsOfClass` "Drone_C"))
        (for _array_element _outactors
          (if (!= _array_element self)
            (`KismetArrayLibrary.Array_Add` (`local.IgnoreActors`) _array_element))))
      (:`then_1`
        (for _array_element_2 (`self.PointLocations`)
          (bind (_outhit _returnvalue) (`KismetSystemLibrary.CapsuleTraceSingle` _array_element_2 (`self.K2_GetActorLocation`) _outradius _outhalfheight "TraceTypeQuery2" false (`local.IgnoreActors`) "None" false (struct :`G` 0.777619 :`B` 1.0 :`A` 1.0) (struct :`R` 1.0 :`G` 1.0 :`B` 1.0 :`A` 1.0)))
          (if _returnvalue
            (if (== (`.HitActor` (`GameplayStatics.BreakHitResult` _outhit)) self)
              (`KismetArrayLibrary.Array_Add` (`local.nLoc`) _array_element_2)
              (`KismetArrayLibrary.Array_Clear` (`self.PointLocations`))
              (bind (_arrayindex _arrayelement) (`/Engine/EditorBlueprintResources/StandardMacros.ReverseForEachLoop` (`local.nLoc`))
                (:`LoopBody`
                  (`KismetArrayLibrary.Array_Add` (`self.PointLocations`) _arrayelement)))
              (else
                (`KismetArrayLibrary.Array_Add` (`local.nLoc`) _array_element_2)))))))))

(fn `SearchRoad`
  (params (CurrentLocation :type "Vector Structure") (FinalLocation :type "Vector Structure") (StepNum :type Integer) (LastRotation :type "Rotator Structure"))
  (returns (Success :type Boolean) (LastStepIndex :type Integer))
  (locals (AdditionalLocation :type "Array of Vector Structure"))
  (bind _currentlocation (`local.CurrentLocation`))
  (bind (_outradius _outhalfheight) (`CapsuleComponent.GetScaledCapsuleSize` (`self.CapsuleComponent`)))
  (bind (_outradius_2 _outhalfheight_2) (`CapsuleComponent.GetScaledCapsuleSize` (`self.CapsuleComponent`)))
  (`|ExecutionSequence`
    (:`then_0`
      (if (>= StepNum (`self.MaxSearchSteps`))
        (return false (`local.StepNum`))))
    (:`then_1`
      (bind (_outhit _returnvalue) (`KismetSystemLibrary.CapsuleTraceSingle` :`Start` CurrentLocation :`End` (+ (`local.CurrentLocation`) (* (`KismetMathLibrary.GetForwardVector` (`KismetMathLibrary.FindLookAtRotation` (`local.CurrentLocation`) (`local.FinalLocation`))) (`self.SearchDist`))) :`Radius` (+ _outradius_2 5.0) :`HalfHeight` (+ _outhalfheight_2 5.0) :`TraceChannel` "TraceTypeQuery1" :`DrawDebugType` (`self.Dl`) :`TraceColor` (`self.GetLinecolor` (`local.StepNum`)) :`DrawTime` 2.0))
      (if _returnvalue
        (bind (_bblockinghit _binitialoverlap _time _distance _location _impactpoint _normal _impactnormal _physmat _hitactor _hitcomponent _hitbonename _hititem _faceindex _tracestart _traceend) (`GameplayStatics.BreakHitResult` _outhit))
        (if (`ActorComponent.ComponentHasTag` _hitcomponent "Point")
          (`KismetArrayLibrary.Array_Add` (`self.PointLocations`) (`local.CurrentLocation`))
          (return true (`local.StepNum`))
          (else
            (for _index (range 1 (+ (`self.SearchInWidthNum`) 1))
              (bind _isa (`/Engine/EditorBlueprintResources/StandardMacros.FlipFlop`)
                (:`A`
                  _)
                (:`B`
                  _))
              (bind (_outhit_2 _returnvalue_2) (`KismetSystemLibrary.CapsuleTraceSingle` :`Start` _currentlocation :`End` (+ _currentlocation (`KismetMathLibrary.RotateAngleAxis` (* (`KismetMathLibrary.GetForwardVector` (`KismetMathLibrary.RLerp` (`KismetMathLibrary.FindLookAtRotation` (`local.CurrentLocation`) (`local.FinalLocation`)) (`local.LastRotation`) 0.5 true)) (`self.SearchDist`)) (* (`KismetMathLibrary.Conv_IntToDouble` _index) (`self.SearchInWidthRadius`) (select `bool` _isa :`false` -1.0 :`true` 1.0 :!type "Float (single-precision)")) (`self.GetActorUpVector`))) :`Radius` _outradius :`HalfHeight` _outhalfheight :`TraceChannel` "TraceTypeQuery1" :`DrawDebugType` (`self.Dl`) :`TraceColor` (`self.GetLinecolor` 0) :`DrawTime` 2.0))
              (if _returnvalue_2
                (bind (_bblockinghit_2 _binitialoverlap_2 _time_2 _distance_2 _location_2 _impactpoint_2 _normal_2 _impactnormal_2 _physmat_2 _hitactor_2 _hitcomponent_2 _hitbonename_2 _hititem_2 _faceindex_2 _tracestart_2 _traceend_2) (`GameplayStatics.BreakHitResult` _outhit_2))
                (if (`ActorComponent.ComponentHasTag` _hitcomponent_2 "Point")
                  (`KismetArrayLibrary.Array_Add` (`self.PointLocations`) (`local.CurrentLocation`))
                  (return true (`local.StepNum`))
                  (elif (>= (`KismetMathLibrary.Vector_Distance2D` _impactpoint_2 (`local.CurrentLocation`)) (`CapsuleComponent.GetScaledCapsuleSize` (`self.CapsuleComponent`)))
                    (`KismetArrayLibrary.Array_Add` (`local.AdditionalLocation`) _impactpoint_2)))
                (else
                  (bind (_success _laststepindex) (`self.SearchRoad` _traceend_2 (`local.FinalLocation`) (+ (`local.StepNum`) 1) (`KismetMathLibrary.FindLookAtRotation` _tracestart_2 _traceend_2)))
                  (`|ExecutionSequence`
                    (:`then_0`
                      (if _success
                        (`KismetArrayLibrary.Array_Add` (`self.PointLocations`) (`local.CurrentLocation`))))
                    (:`then_1`
                      (return _success _laststepindex))))))
            (if (> (`KismetArrayLibrary.Array_Length` (`local.AdditionalLocation`)) 0)
              (for _array_element (`local.AdditionalLocation`)
                (bind (_success_2 _laststepindex_2) (`self.SearchRoad` _array_element (`local.FinalLocation`) (+ (`local.StepNum`) 1)))
                (return _success_2 _laststepindex_2)))
            (return false (`local.StepNum`))))
        (else
          (bind (_success_3 _laststepindex_3) (`self.SearchRoad` _traceend (`local.FinalLocation`) (+ (`local.StepNum`) 1) (`KismetMathLibrary.FindLookAtRotation` _tracestart _traceend)))
          (`|ExecutionSequence`
            (:`then_0`
              (if _success_3
                (`KismetArrayLibrary.Array_Add` (`self.PointLocations`) (`local.CurrentLocation`))))
            (:`then_1`
              (return _success_3 _laststepindex_3))))))))

(fn `SpawnPoints`
  (params (Location :type "Vector Structure"))
  (bind _returnvalue (`|SpawnActorFromClass` "/Game/Test1/Blueprint/Objects/Point.Point_C" (`KismetMathLibrary.MakeTransform` Location (struct) (0.5 0.5 0.5)) "Undefined" "OverrideRootScale" null null))
  (`KismetArrayLibrary.Array_Add` (`self.Points`) _returnvalue)
  (`self.SetActorEnableCollision` _returnvalue false))

(fn `UserConstructionScript`)